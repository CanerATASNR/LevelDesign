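; BP_Interaction shows an interaction text label in the world through its Widget component.
; On BeginPlay it creates a WB_InteractionText widget from its TextContent value and assigns it to that component.
; Every Tick it rotates the component toward the first player character's camera, so the text always faces the player.
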(event `self.ReceiveBeginPlay`
  (bind _returnvalue (`|CreateWidget` "/Game/Development/UI/WB_InteractionText.WB_InteractionText_C" null (`self.TextContent`)))
  (`WidgetComponent.SetWidget` (`self.Widget`) _returnvalue))

(event `self.ReceiveTick`
  (params (DeltaSeconds :type "Float (single-precision)"))
  (bind _widget (`self.Widget`))
  (`SceneComponent.K2_SetWorldRotation` _widget (`KismetMathLibrary.FindLookAtRotation` (`SceneComponent.K2_GetComponentLocation` _widget) (`SceneComponent.K2_GetComponentLocation` (`self.GetComponentByClass` (`GameplayStatics.GetPlayerCharacter` 0) "/Script/Engine.CameraComponent"))) false false))

(fn `UserConstructionScript`)