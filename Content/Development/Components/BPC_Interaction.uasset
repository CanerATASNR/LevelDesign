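; BPC_Interaction is an actor component that gives its owning actor outline highlight feedback for interaction.
; InArea applies the MI_Outline overlay material to the owner's static mesh component and OutArea clears it, both only on the Active branch of a TutorialState switch.
; Looking and NotLooking currently only log the owner's name, with no visual effect.
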(event `/Game/Development/Comm/BPI_ınteraction.InArea`
  ;[0.15 0.15 0.15 0.5 12] Alan Kontrolü
  ;;[0.15 0.15 0.15 0.5 12] Alana girdi kontrolü
  (`/Game/Development/Global/GlobalMacros.SwitchonTutorialState`
    (:`Active`
      (`MeshComponent.SetOverlayMaterial` (`Actor.GetComponentByClass` (`self.GetOwner`) "/Script/Engine.StaticMeshComponent") "/Game/Art/Materials/Base/MI_Outline.MI_Outline") ; Overlay materyalini ayarla (outline)
    )))

(event `/Game/Development/Comm/BPI_ınteraction.OutArea`
  ;[0.15 0.15 0.15 0.5 12] Alan Kontrolü
  ;;[0.15 0.15 0.15 0.5 12] Alandan çıktı kontrolü
  (`/Game/Development/Global/GlobalMacros.SwitchonTutorialState`
    (:`Active`
      (`MeshComponent.SetOverlayMaterial` (`Actor.GetComponentByClass` (`self.GetOwner`) "/Script/Engine.StaticMeshComponent") null) ; Overlay materyalini ayarla (boş)
    )))

(event `/Game/Development/Comm/BPI_ınteraction.Looking`
  (`KismetSystemLibrary.LogString` (`KismetStringLibrary.BuildString_Object` "Looking on: " "" (`self.GetOwner`))))

(event `/Game/Development/Comm/BPI_ınteraction.NotLooking`
  (`KismetSystemLibrary.LogString` (`KismetStringLibrary.BuildString_Object` "Not looking on: " "" (`self.GetOwner`))))