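; Interaction component that highlights its owning actor for the player and shows a "Press E" prompt.
; InArea caches each static mesh's first material, applies MI_Outline and sends BeginTraceMessage to the player; OutArea restores materials by index and sends EndTraceMessage.
; LookingNow enables owner input and spawns a BP_Interaction prompt with the owner's name above it.
; NotLooking disables input and destroys that prompt.
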(event `/Game/Development/Comm/BPI_Interaction.InArea`
  (bind _returnvalue (`Actor.K2_GetComponentsByClass` (`self.GetOwner`) "/Script/Engine.StaticMeshComponent"))
  (for _array_element _returnvalue
    (`KismetArrayLibrary.Array_Add` (`self.Materials`) (`PrimitiveComponent.GetMaterial` _array_element 0)))
  (`PrimitiveComponent.SetMaterial` _returnvalue 0 "/Game/Art/Materials/MI_Outline.MI_Outline")
  (message `/Game/Development/Comm/BPI_Interaction.BeginTrace` (`GameplayStatics.GetPlayerCharacter` 0)))

(event `/Game/Development/Comm/BPI_Interaction.OutArea`
  (for (_array_element _array_index) (`Actor.K2_GetComponentsByClass` (`self.GetOwner`) "/Script/Engine.StaticMeshComponent")
    (`PrimitiveComponent.SetMaterial` _array_element 0 (`|GetArrayItem` (`self.Materials`) _array_index)))
  (message `/Game/Development/Comm/BPI_Interaction.EndTrace` (`GameplayStatics.GetPlayerCharacter` 0)))

(event `/Game/Development/Comm/BPI_Interaction.LookingNow`
  (bind _returnvalue (`self.GetOwner`))
  (bind (_returnvalue_x _returnvalue_y _returnvalue_z) (`KismetMathLibrary.BreakVector` (`Actor.K2_GetActorLocation` _returnvalue)))
  ;[0.15 0.15 0.15 0.5 12] Area Control
  (`Actor.EnableInput` _returnvalue (`GameplayStatics.GetPlayerController` 0))
  (bind _returnvalue_2 (`|SpawnActorFromClass` "/Game/Development/System/BP_Interaction.BP_Interaction_C" (`KismetMathLibrary.MakeTransform` (`KismetMathLibrary.MakeVector` _returnvalue_x _returnvalue_y (+ _returnvalue_z 50.0))) "Undefined" "MultiplyWithRoot" null (`KismetTextLibrary.Conv_StringToText` (`KismetStringLibrary.BuildString_Name` "Press \"E\" to interact with " "" (`KismetStringLibrary.Conv_StringToName` (`KismetSystemLibrary.GetDisplayName` _returnvalue)))) null)))

(event `/Game/Development/Comm/BPI_Interaction.NotLooking`
  ;[0.15 0.15 0.15 0.5 12] Area Control
  (`Actor.DisableInput` (`self.GetOwner`) (`GameplayStatics.GetPlayerController` 0))
  (`Actor.K2_DestroyActor` (stale `/Game/Development/Comm/BPI_Interaction.LookingNow` _returnvalue_2)))